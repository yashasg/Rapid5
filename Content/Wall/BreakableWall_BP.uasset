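; BreakableWall_BP is a wall that breaks when an actor tagged "Car" hits it.
; On each such hit it spawns a ColorWall actor at its own transform and applies damage to its Destructible component.
; It then gets player 0's GameHUD and increments the boost count there, with no guard against repeat hits.
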(event `self.ReceiveHit`
  (params (MyComp :type "PrimitiveComponent Object Reference") (Other :type "Actor Object Reference") (OtherComp :type "PrimitiveComponent Object Reference") (bSelfMoved :type Boolean) (HitLocation :type "Vector Structure") (HitNormal :type "Vector Structure") (NormalImpulse :type "Vector Structure") (Hit :type "HitResult Structure (by ref)"))
  (if (`self.ActorHasTag` Other "Car")
    (`|SpawnActorFromClass` "/Game/Wall/ColorWall.ColorWall_C" (`self.GetTransform`) "Undefined" "OverrideRootScale")
    (`DestructibleComponent.ApplyDamage` (`self.Destructible`) 1.0 (`KismetMathLibrary.MakeVector` 0.0) (`KismetMathLibrary.MakeVector` 0.0) 0.0)
    (bind _asgame_hud (cast `/Game/Blueprints/GameHUD` (`PlayerController.GetHUD` (`GameplayStatics.GetPlayerController` 0))))
    (`/Game/Blueprints/GameHUD.BoostCountInc` _asgame_hud)))

(fn `UserConstructionScript`)