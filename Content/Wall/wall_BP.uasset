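; Wall Blueprint that reacts when an actor tagged "Car" hits it with a collapse sound, a timed explosion particle effect and a Boost increment.
; On hit it disables gravity on its own hit component, then casts the other actor to VehicleBlueprint to reach Boost and the spring arm.
; A brief global slow-motion beat plays while the car's spring arm swings the camera around, then time and camera angle are set back.
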(event `self.ReceiveHit`
  (params (MyComp :type "PrimitiveComponent Object Reference") (Other :type "Actor Object Reference") (OtherComp :type "PrimitiveComponent Object Reference") (bSelfMoved :type Boolean) (HitLocation :type "Vector Structure") (HitNormal :type "Vector Structure") (NormalImpulse :type "Vector Structure") (Hit :type "HitResult Structure (by ref)"))
  (if (`self.ActorHasTag` Other "Car")
    (`GameplayStatics.PlaySound2D` "/Game/StarterContent/Audio/Collapse_Cue.Collapse_Cue")
    (`PrimitiveComponent.SetEnableGravity` MyComp false)
    (`self.EnableParticleSystem`)
    (bind _asvehicle_blueprint (cast `/Game/VehicleAdvBP/Blueprints/VehicleBlueprint` Other))
    (set `/Game/VehicleAdvBP/Blueprints/VehicleBlueprint.Boost` (+ (`/Game/VehicleAdvBP/Blueprints/VehicleBlueprint.Boost` _asvehicle_blueprint) 1) _asvehicle_blueprint)
    (`self.RotateCamera`)
    (`GameplayStatics.SetGlobalTimeDilation` 0.2)
    (`KismetSystemLibrary.Delay` 0.25)
    (`GameplayStatics.SetGlobalTimeDilation` 1.0)
    (`self.Reset Camera`)))

(event `EnableParticleSystem`
  (bind _returnvalue (`GameplayStatics.SpawnEmitterAtLocation` "/Game/StarterContent/Particles/New_Particle_Effects/P_Explosion_Psy.P_Explosion_Psy" (stale `self.ReceiveHit` HitLocation) (struct) false))
  (`KismetSystemLibrary.Delay` 2.0)
  (`ActorComponent.K2_DestroyComponent` _returnvalue))

(event `RotateCamera`
  (`SceneComponent.K2_SetRelativeRotation` (`/Game/VehicleAdvBP/Blueprints/VehicleBlueprint.SpringArm` (stale `self.ReceiveHit` _asvehicle_blueprint)) (struct :`Yaw` -180.0) true false))

(event `Reset Camera`
  (`SceneComponent.K2_SetRelativeRotation` (`/Game/VehicleAdvBP/Blueprints/VehicleBlueprint.SpringArm` (stale `self.ReceiveHit` _asvehicle_blueprint)) (struct :`Pitch` -30.0) true false))

(fn `UserConstructionScript`)