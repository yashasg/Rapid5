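; GameHUD is a HUD Blueprint that draws the elapsed time and the player vehicle's boost count on screen.
; On BeginPlay it resets its game variables and starts a looping timer that calls Clock, which increments StoreTime on the TransferInstance GameInstance.
; DrawHUD prints that time and copies Boost from the owning VehicleBlueprint pawn into the GameInstance before displaying it.
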(event `Clock`
  (bind _astransfer_instance (cast `/Game/TransferInstance` (`GameplayStatics.GetGameInstance`)))
  (bind _output_get (set `/Game/TransferInstance.StoreTime` (+ (`/Game/TransferInstance.StoreTime` _astransfer_instance) 0.01) _astransfer_instance)))

(event `self.ReceiveBeginPlay`
  (`self.StartGame`))

(event `self.ReceiveDrawHUD`
  (params (SizeX :type Integer) (SizeY :type Integer))
  (`self.DrawText` (`KismetStringLibrary.Concat_StrStr` "Time: " (`KismetStringLibrary.TimeSecondsToString` (stale `Clock` _output_get))) (struct :`R` 0.795 :`G` 0.179 :`B` 0.179 :`A` 1.0) 0.0 0.0 null 3.0)
  (bind _asvehicle_blueprint (cast `/Game/VehicleAdvBP/Blueprints/VehicleBlueprint` (`self.GetOwningPawn`)))
  (bind _output_get (set `/Game/TransferInstance.StoreBoost` (`/Game/VehicleAdvBP/Blueprints/VehicleBlueprint.Boost` _asvehicle_blueprint) (stale `Clock` _astransfer_instance)))
  (`self.DrawText` (`KismetStringLibrary.Concat_StrStr` "Boost x" (`KismetStringLibrary.Conv_IntToString` _output_get)) (struct :`R` 0.975 :`G` 0.975 :`B` 0.975 :`A` 1.0) 50.0 50.0 null 2.0))

(event `self.ReceiveActorBeginOverlap`
  (params (OtherActor :type "Actor Object Reference")))

(event `self.ReceiveTick`
  (params (DeltaSeconds :type "Float (single-precision)")))

(fn `UserConstructionScript`)